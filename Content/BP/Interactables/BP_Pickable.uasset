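; BP_Pickable is an interactable world item that reports itself as an item rather than a chest or crafting station.
; Its Interact function calls the parent implementation before returning that type, while its Equip function returns no placement.
; On BeginPlay, an optional DisableCollision flag turns off actor collision and mesh physics and makes the mesh ignore the Visibility channel.
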(event `self.ReceiveBeginPlay`
  (bind _staticmeshcomponent (`self.StaticMeshComponent`))
  (if (`self.DisableCollision`)
    (`self.SetActorEnableCollision` false)
    (`PrimitiveComponent.SetSimulatePhysics` _staticmeshcomponent false)
    (`PrimitiveComponent.SetCollisionResponseToChannel` _staticmeshcomponent "ECC_Visibility" "ECR_Ignore")))

(fn `F_Equip`
  (returns (`Placement?` :type Boolean) (Class :type "/Game/BP/Interactables/Seed/Plants/BP_Placeble Class Reference"))
  (return false null))

(fn `I_Interact`
  (returns (`Item?` :type Boolean) (`Chest?` :type Boolean) (`CraftingStation?` :type Boolean) (ChestRef :type "Actor Object Reference") (CraftingStation :type "GameplayTag Structure"))
  (`parent.I_Interact`)
  (return true false false null))

(fn `UserConstructionScript`
  (`parent.UserConstructionScript`))