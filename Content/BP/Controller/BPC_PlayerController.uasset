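; Player controller that feeds Enhanced Input move, look, jump and interact actions to the possessed BP_Player.
; BeginPlay adds the IMC_Player mapping context and caches the pawn as OwnerRef, with movement following control yaw only.
; A short camera-forward sphere trace runs on interact, and on Tick while ShouldCheckForInteraction is set.
; The trace draws debug shapes, but its hit result is not used yet.
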(event `ke_CheckInteractInSight`
  (if (`self.ShouldCheckForInteraction`)
    (`self.AimTraceFromPlayer` 200.0 4.0 "ForOneFrame" 0.0)))

(event `self.ReceiveTick`
  (params (DeltaSeconds :type "Float (single-precision)"))
  (`self.ke_CheckInteractInSight`))

(event `EnhancedInput|/Game/BP/Input/IA_Move`
  (params (ActionValue :type "Vector2D Structure") (ElapsedSeconds :type "Float (double-precision)") (TriggeredSeconds :type "Float (double-precision)") (InputAction :type "InputAction Object Reference" :default "/Game/BP/Input/IA_Move.IA_Move"))
  (bind (_returnvalue_roll _returnvalue_pitch _returnvalue_yaw) (`KismetMathLibrary.BreakRotator` (`Pawn.GetControlRotation` (`self.OwnerRef`))))
  (bind _returnvalue (`KismetMathLibrary.MakeRotator` 0.0 0.0 _returnvalue_yaw))
  ;[0.04167 0.04167 0.04167] Base Movement and Camera input
  (:`Triggered`
    (`Pawn.AddMovementInput` (`self.OwnerRef`) (`KismetMathLibrary.GetRightVector` _returnvalue) ActionValue_X false)
    (`Pawn.AddMovementInput` (`self.OwnerRef`) (`KismetMathLibrary.GetForwardVector` _returnvalue) ActionValue_Y false)))

(event `EnhancedInput|/Game/BP/Input/IA_CameraMove`
  (params (ActionValue :type "Vector2D Structure") (ElapsedSeconds :type "Float (double-precision)") (TriggeredSeconds :type "Float (double-precision)") (InputAction :type "InputAction Object Reference" :default "/Game/BP/Input/IA_CameraMove.IA_CameraMove"))
  ;[0.04167 0.04167 0.04167] Base Movement and Camera input
  (:`Triggered`
    (`Pawn.AddControllerYawInput` (`self.OwnerRef`) ActionValue_X)
    (`Pawn.AddControllerPitchInput` (`self.OwnerRef`) ActionValue_Y)))

(event `EnhancedInput|/Game/BP/Input/IA_Jump`
  (params (ActionValue :type Boolean) (ElapsedSeconds :type "Float (double-precision)") (TriggeredSeconds :type "Float (double-precision)") (InputAction :type "InputAction Object Reference" :default "/Game/BP/Input/IA_Jump.IA_Jump"))
  ;[0.04167 0.04167 0.04167] Base Movement and Camera input
  (:`Triggered`
    (`Character.Jump` (`self.OwnerRef`)))
  (:`Canceled`
    (`Character.StopJumping` (`self.OwnerRef`) :!label _label))
  (:`Completed`
    (goto _label)))

(event `EnhancedInput|/Game/BP/Input/IA_Interact`
  (params (ActionValue :type Boolean) (ElapsedSeconds :type "Float (double-precision)") (TriggeredSeconds :type "Float (double-precision)") (InputAction :type "InputAction Object Reference" :default "/Game/BP/Input/IA_Interact.IA_Interact"))
  ;[0.04167 0.04167 0.04167] Interact Input
  (:`Triggered`
    (`self.AimTraceFromPlayer` 200.0 4.0 "ForDuration")))

(event `self.ReceiveBeginPlay`
  ;[0.04167 0.04167 0.04167] Setup Reference and start mapping input
  (`EnhancedInputSubsystemInterface.AddMappingContext` (subsystem `EnhancedInputLocalPlayerSubsystem`) "/Game/BP/Input/IMC_Player.IMC_Player" 0 (struct))
  (bind _asbp_player (cast `/Game/BP/Character/PlayerCharacter/BP_Player` (`self.K2_GetPawn`)))
  (set `self.OwnerRef` _asbp_player))

(fn `AimTraceFromPlayer`
  (params (TraceLength :type "Float (single-precision)" :default 400.0) (Radius :type "Float (single-precision)" :default 6.0) (DrawDebugType :type "EDrawDebugTrace Enum" :default "None") (DrawTime :type "Float (single-precision)" :default 0.01))
  (bind _returnvalue (`GameplayStatics.GetPlayerCameraManager` 0))
  (bind _returnvalue_2 (`PlayerCameraManager.GetCameraLocation` _returnvalue))
  (`KismetSystemLibrary.SphereTraceSingle` :`Start` _returnvalue_2 :`End` (+ _returnvalue_2 (* (`self.GetActorForwardVector` _returnvalue) TraceLength)) :`Radius` Radius :`TraceChannel` "TraceTypeQuery1" :`DrawDebugType` DrawDebugType :`DrawTime` DrawTime))

(fn `UserConstructionScript`)