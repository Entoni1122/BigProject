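; BP_Chest is an interactable loot chest that holds a 12-slot item inventory with randomized contents.
; On BeginPlay the server creates empty slots, then fills a random number from DT_RandomChest rows, with amounts based on each item tag's stack size.
; Events remove, move, merge, add or resize slot entries.
; The I_GetChest interface returns the chest only while IsOpen is false.
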(event `self.ReceiveBeginPlay`
  (if (`KismetSystemLibrary.IsServer`)
    (for _ (range 12)
      (`KismetArrayLibrary.Array_Add` (`self.Items`) (make `/Game/BP/Structs/SlotData` (struct))))
    (bind _output_get (set `self.RandomAmountItem` (`KismetMathLibrary.RandomIntegerInRange` 1 11)))
    (bind _outrownames (`DataTableFunctionLibrary.GetDataTableRowNames` "/Game/BP/Datatables/DT_RandomChest.DT_RandomChest"))
    (for _index (range _output_get)
      (bind _returnvalue (`|GetDataTableRow` "/Game/BP/Datatables/DT_RandomChest.DT_RandomChest" (`KismetArrayLibrary.Array_Random` _outrownames))
        (:`then`
          (bind _itemstack (`/Game/BP/Functions/CustomLibrary.GetStackFromTag` (break `/Game/BP/Structs/ObjectData` _returnvalue)))
          (`KismetArrayLibrary.Array_Set` (`self.Items`) _index (make `/Game/BP/Structs/SlotData` (break `/Game/BP/Structs/ObjectData` _returnvalue) (`KismetMathLibrary.SelectInt` (`KismetMathLibrary.RandomIntegerInRange` 1 (- _itemstack 1)) 1 (> _itemstack 1)) _itemstack)))))))

(event `RemoveItem`
  (params (SlotIndex :type Integer))
  (`KismetArrayLibrary.Array_Set` (`self.Items`) SlotIndex (make `/Game/BP/Structs/SlotData` (struct))))

(event `AddAmountInternal`
  (params (SelectedSlotIndex :type Integer) (DropSlotIndex :type Integer) (AdditiveAmount :type Integer) (Stack :type Integer))
  (bind (_output_item _output_amount _output_stack) (break `/Game/BP/Structs/SlotData` (`|GetArrayItem` (`self.Items`) SelectedSlotIndex)))
  (if (< AdditiveAmount Stack)
    (`KismetArrayLibrary.Array_Set` (`self.Items`) DropSlotIndex (make `/Game/BP/Structs/SlotData` _output_item AdditiveAmount _output_stack))
    (`KismetArrayLibrary.Array_Set` (`self.Items`) SelectedSlotIndex (make `/Game/BP/Structs/SlotData` (struct)))
    (else
      (`KismetArrayLibrary.Array_Set` (`self.Items`) DropSlotIndex (make `/Game/BP/Structs/SlotData` _output_item _output_stack _output_stack))
      (`KismetArrayLibrary.Array_Set` (`self.Items`) SelectedSlotIndex (make `/Game/BP/Structs/SlotData` _output_item (- AdditiveAmount Stack) _output_stack)))))

(event `SwapItem`
  (params (SelectedIndex :type Integer) (DropIndex :type Integer))
  (`KismetArrayLibrary.Array_Set` (`self.Items`) DropIndex (`|GetArrayItem` (`self.Items`) SelectedIndex))
  (`KismetArrayLibrary.Array_Set` (`self.Items`) SelectedIndex (make `/Game/BP/Structs/SlotData` (struct))))

(event `AddItemToEmptySlot`
  (params (SelectedSlotIndex :type Integer) (Item :type "/Game/BP/Structs/SlotData Structure (by ref)"))
  (`KismetArrayLibrary.Array_Set` (`self.Items`) SelectedSlotIndex Item))

(event `SetAmountAtIndex`
  (params (Index :type Integer) (Amount :type Integer))
  (bind (_output_item _output_amount _output_stack) (break `/Game/BP/Structs/SlotData` (`|GetArrayItem` (`self.Items`) Index)))
  (`KismetArrayLibrary.Array_Set` (`self.Items`) Index (make `/Game/BP/Structs/SlotData` _output_item Amount _output_stack)))

(fn `I_GetChest`
  (returns (Chest :type "Actor Object Reference"))
  (if (`self.IsOpen?`)
    (return null)
    (else
      (return self))))

(fn `I_Pickup`
  (return))

(fn `UserConstructionScript`)