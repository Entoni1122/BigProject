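; Placeable plant actor that previews whether it can be placed, then grows once placed.
; A dynamic material instance shows build mode, with CheckForCollision overlaps toggling its can't-build parameter and the CanBePlace flag.
; ItemInPlace destroys that check and starts a looping timer that scales the actor up until PlaceTime, then enables collision.
; Its pickup interface function simply returns true.
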(event `self.ReceiveBeginPlay`
  (`PrimitiveComponent.SetSimulatePhysics` (`self.StaticMeshComponent`) false)
  (`self.SetActorEnableCollision` false)
  (bind _returnvalue (`PrimitiveComponent.CreateDynamicMaterialInstance` (`self.StaticMeshComponent`) 0 "/Game/Materials/MI_TestPlant.MI_TestPlant" "None"))
  (bind _output_get (set `self.DynMat` _returnvalue))
  (`MaterialInstanceDynamic.SetScalarParameterValue` _output_get "BuildOn" 1.0)
  (`MaterialInstanceDynamic.SetScalarParameterValue` _output_get "CantBuild?" 0.0))

(event `self.CheckForCollision.OnComponentBeginOverlap`
  (params (OverlappedComponent :type "PrimitiveComponent Object Reference") (OtherActor :type "Actor Object Reference") (OtherComp :type "PrimitiveComponent Object Reference") (OtherBodyIndex :type Integer) (bFromSweep :type Boolean) (SweepResult :type "HitResult Structure (by ref)"))
  (bind _dynmat (`self.DynMat`)
    (:`then`
      (`MaterialInstanceDynamic.SetScalarParameterValue` _dynmat "CantBuild?" 1.0)
      (set `self.CanBePlace?` false))
    (:`else`)))

(event `self.CheckForCollision.OnComponentEndOverlap`
  (params (OverlappedComponent :type "PrimitiveComponent Object Reference") (OtherActor :type "Actor Object Reference") (OtherComp :type "PrimitiveComponent Object Reference") (OtherBodyIndex :type Integer))
  (bind _dynmat (`self.DynMat`)
    (:`then`
      (`MaterialInstanceDynamic.SetScalarParameterValue` _dynmat "CantBuild?" 0.0)
      (set `self.CanBePlace?` true))
    (:`else`)))

(event `ItemInPlace`
  (`ActorComponent.K2_DestroyComponent` (`self.CheckForCollision`))
  (bind _returnvalue (`KismetSystemLibrary.K2_SetTimerDelegate` (delegate `GrowTime`) 1.0 true -1.0)))

(event `GrowTime`
  (set `self.CurrentTime` (+ (`self.CurrentTime`) 1.0))
  (`self.SetActorScale3D` (* (1.0 1.0 1.0) (/ (`self.CurrentTime`) (`self.PlaceTime`))))
  (if (>= (`self.CurrentTime`) (`self.PlaceTime`))
    (`self.SetActorEnableCollision` true)
    (`KismetSystemLibrary.K2_ClearAndInvalidateTimerHandle` (stale `ItemInPlace` _returnvalue))))

(fn `I_Pickup`
  (returns (`Item?` :type Boolean))
  (return true))

(fn `UserConstructionScript`
  (`parent.UserConstructionScript`))