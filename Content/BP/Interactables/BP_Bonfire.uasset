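; BP_Bonfire is an interactable bonfire that takes cooking requests through the I_Cook interface.
; ICook accepts an item only if it passes the cookable check and the spawned-food counter is below its maximum, returning whether it was accepted.
; Accepted items go to the Cook event, which only prints a debug string; no food is spawned and the counter is never incremented here.
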(event `Cook`
  (params (FoodToBeCooked :type "GameplayTag Structure"))
  (`KismetSystemLibrary.PrintString` "Cook"))

(fn `I_Cook`
  (params (ItemToBeCooked :type "GameplayTag Structure"))
  (returns (Return :type Boolean))
  (if (`/Game/BP/Functions/CustomLibrary.IsCookableItem?` ItemToBeCooked)
    (if (< (`self.FoodSpawnedCounter`) (`self.MaxSpawnableFood`))
      (`self.Cook` (`local.ItemToBeCooked`))
      (return true)
      (else
        (return false)))
    (else
      (return false))))

(fn `UserConstructionScript`
  (`parent.UserConstructionScript`))