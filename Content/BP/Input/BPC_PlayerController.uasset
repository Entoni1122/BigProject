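; BPC_PlayerController is the player controller that turns Enhanced Input actions into movement, camera look and jumping on the possessed BP_Player.
; On BeginPlay it adds the IMC_Player mapping context, then casts the controlled pawn to BP_Player and caches it as OwnerRef.
; Input events forward to that cached pawn, with movement directions taken from control yaw only so camera pitch does not affect them.
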(event `self.ReceiveBeginPlay`
  (`EnhancedInputSubsystemInterface.AddMappingContext` (subsystem `EnhancedInputLocalPlayerSubsystem`) "/Game/BP/Input/IMC_Player.IMC_Player" 0 (struct))
  (bind _asbp_player (cast `/Game/BP/Character/PlayerCharacter/BP_Player` (`self.K2_GetPawn`)))
  (set `self.OwnerRef` _asbp_player))

(event `EnhancedInput|/Game/BP/Input/IA_Move`
  (params (ActionValue :type "Vector2D Structure") (ElapsedSeconds :type "Float (double-precision)") (TriggeredSeconds :type "Float (double-precision)") (InputAction :type "InputAction Object Reference" :default "/Game/BP/Input/IA_Move.IA_Move"))
  (bind _ownerref (`self.OwnerRef`))
  (bind (_returnvalue_roll _returnvalue_pitch _returnvalue_yaw) (`KismetMathLibrary.BreakRotator` (`Pawn.GetControlRotation` _ownerref)))
  (bind _returnvalue (`KismetMathLibrary.MakeRotator` 0.0 0.0 _returnvalue_yaw))
  ;[1 1 1] Movemnt
  (:`Triggered`
    (`Pawn.AddMovementInput` _ownerref (`KismetMathLibrary.GetRightVector` _returnvalue) ActionValue_X false)
    (`Pawn.AddMovementInput` (`self.OwnerRef`) (`KismetMathLibrary.GetForwardVector` _returnvalue) ActionValue_Y false)))

(event `EnhancedInput|/Game/BP/Input/IA_CameraMove`
  (params (ActionValue :type "Vector2D Structure") (ElapsedSeconds :type "Float (double-precision)") (TriggeredSeconds :type "Float (double-precision)") (InputAction :type "InputAction Object Reference" :default "/Game/BP/Input/IA_CameraMove.IA_CameraMove"))
  (bind _ownerref (`self.OwnerRef`))
  ;[1 1 1] Movemnt
  (:`Triggered`
    (`Pawn.AddControllerYawInput` _ownerref ActionValue_X)
    (`Pawn.AddControllerPitchInput` _ownerref ActionValue_Y)))

(event `EnhancedInput|/Game/BP/Input/IA_Jump`
  (params (ActionValue :type Boolean) (ElapsedSeconds :type "Float (double-precision)") (TriggeredSeconds :type "Float (double-precision)") (InputAction :type "InputAction Object Reference" :default "/Game/BP/Input/IA_Jump.IA_Jump"))
  ;[1 1 1] Movemnt
  (:`Triggered`
    (`Character.Jump` (`self.OwnerRef`))))

(fn `UserConstructionScript`)