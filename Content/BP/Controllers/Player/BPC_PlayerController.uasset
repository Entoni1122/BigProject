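; Player controller that maps Enhanced Input to BP_Player movement, camera, jump, stamina-gated running, inventory toggle and interaction.
; Each tick, a camera sphere trace finds "Interactable"-tagged actors, stores the target and shows its tag on the HUD.
; Interacting sends pickable item data to the HUD's inventory widget, updating the pickable when adding fails.
; Server-named events handle run-speed changes (relayed to a multicast), item data updates and spawning dropped items before the player.
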(event `ke_CheckInteractInSight`
  (bind _hudref (`self.HUDRef`))
  (if (`self.ShouldCheckForInteraction`)
    (bind (_returnvalue _outhit) (`self.AimTraceFromPlayer` 200.0 4.0 "None" 0.0))
    (if _returnvalue
      (bind (_bblockinghit _binitialoverlap _time _distance _location _impactpoint _normal _impactnormal _physmat _hitactor) (`GameplayStatics.BreakHitResult` _outhit))
      (if (`self.ActorHasTag` _hitactor "Interactable")
        (`/Engine/EditorBlueprintResources/StandardMacros.IsValid` _hudref
          (:`Is Valid`
            (`/Game/BP/HUDs/BaseHUD.ke_ShowText` _hudref true (`|GetArrayItem` (`Actor.Tags` _hitactor) 1))
            (set `self.InteractableRef` _hitactor)))
        (else
          (`self.InteractableRef` :!label _label
            (:`then`
              (set `self.InteractableRef` null)
              (`/Game/BP/HUDs/BaseHUD.ke_ShowText` (`self.HUDRef`) false "None"))
            (:`else`))))
      (else
        (goto _label)))))

(event `self.ReceiveTick`
  (params (DeltaSeconds :type "Float (single-precision)"))
  (`self.ke_CheckInteractInSight`))

(event `ke_DropItemOnGround`
  (params (ItemInfo :type "/Game/BP/Structs/InteractableInfos Structure"))
  (bind _ownerref (`self.OwnerRef`))
  (`/Engine/EditorBlueprintResources/StandardMacros.IsValid` _ownerref
    (:`Is Valid`
      (`self.SpawnObjOnServer` ItemInfo_Class_10_7A572F6E40143F7CE4FB0789F22795D1 _ownerref))))

(event `SpawnObjOnServer`
  (params (Class :type "Actor Class Reference") (Target :type "Actor Object Reference"))
  (`|SpawnActorFromClass` Class (`KismetMathLibrary.MakeTransform` (+ (`self.K2_GetActorLocation` Target) (* (`self.GetActorForwardVector` Target) 100.0))) "Undefined" "OverrideRootScale" null null))

(event `EnhancedInput|/Game/BP/Inputs/InputActions/IA_Move`
  (params (ActionValue :type "Vector2D Structure") (ElapsedSeconds :type "Float (double-precision)") (TriggeredSeconds :type "Float (double-precision)") (InputAction :type "InputAction Object Reference" :default "/Game/BP/Inputs/InputActions/IA_Move.IA_Move"))
  (bind (_returnvalue_roll _returnvalue_pitch _returnvalue_yaw) (`KismetMathLibrary.BreakRotator` (`Pawn.GetControlRotation` (`self.OwnerRef`))))
  (bind _returnvalue (`KismetMathLibrary.MakeRotator` 0.0 0.0 _returnvalue_yaw))
  ;[0.04167 0.04167 0.04167] Base Movement and Camera input
  (:`Triggered`
    (`Pawn.AddMovementInput` (`self.OwnerRef`) (`KismetMathLibrary.GetRightVector` _returnvalue) ActionValue_X false)
    (`Pawn.AddMovementInput` (`self.OwnerRef`) (`KismetMathLibrary.GetForwardVector` _returnvalue) ActionValue_Y false)))

(event `EnhancedInput|/Game/BP/Inputs/InputActions/IA_CameraMove`
  (params (ActionValue :type "Vector2D Structure") (ElapsedSeconds :type "Float (double-precision)") (TriggeredSeconds :type "Float (double-precision)") (InputAction :type "InputAction Object Reference" :default "/Game/BP/Inputs/InputActions/IA_CameraMove.IA_CameraMove"))
  ;[0.04167 0.04167 0.04167] Base Movement and Camera input
  (:`Triggered`
    (`Pawn.AddControllerYawInput` (`self.OwnerRef`) ActionValue_X)
    (`Pawn.AddControllerPitchInput` (`self.OwnerRef`) ActionValue_Y)))

(event `EnhancedInput|/Game/BP/Inputs/InputActions/IA_Jump`
  (params (ActionValue :type Boolean) (ElapsedSeconds :type "Float (double-precision)") (TriggeredSeconds :type "Float (double-precision)") (InputAction :type "InputAction Object Reference" :default "/Game/BP/Inputs/InputActions/IA_Jump.IA_Jump"))
  ;[0.04167 0.04167 0.04167] Base Movement and Camera input
  (:`Triggered`
    (`Character.Jump` (`self.OwnerRef`)))
  (:`Canceled`
    (`Character.StopJumping` (`self.OwnerRef`) :!label _label))
  (:`Completed`
    (goto _label)))

(event `EnhancedInput|/Game/BP/Inputs/InputActions/IA_Interact`
  (params (ActionValue :type Boolean) (ElapsedSeconds :type "Float (double-precision)") (TriggeredSeconds :type "Float (double-precision)") (InputAction :type "InputAction Object Reference" :default "/Game/BP/Inputs/InputActions/IA_Interact.IA_Interact"))
  ;[0.04167 0.04167 0.04167] Interact Input
  (:`Triggered`
    (bind _interactableref (`self.InteractableRef`)
      (:`then`
        (bind _item_ (message `/Game/BP/Interfaces/Interactablenterface.I_Interact` _interactableref))
        (if _item_
          (bind _asbp_pickable (cast `/Game/BP/Items/BP_Pickable` _interactableref :!pure true))
          (bind (_success_ _newitemdata) (`/Game/BP/Widgets/WDB_Inventory.ke_TryAddItem` (`/Game/BP/Widgets/WDB_HUD.WDB_Inventory` (`/Game/BP/HUDs/BaseHUD.MainWidgetRef` (`self.HUDRef`))) (`/Game/BP/Items/BP_BaseItem.Item Data` _asbp_pickable)))
          (if (not _success_)
            (`self.ServerUpdateItemData` _newitemdata _asbp_pickable))))
      (:`else`))))

(event `ServerUpdateItemData`
  (params (`Item Data` :type "/Game/BP/Structs/InteractableInfos Structure") (Actor :type "/Game/BP/Items/BP_Pickable Object Reference"))
  ;[0.04167 0.04167 0.04167] Interact Input
  (set `/Game/BP/Items/BP_BaseItem.Item Data` `Item Data` Actor))

(event `EnhancedInput|/Game/BP/Inputs/InputActions/IA_ToogleInventory`
  (params (ActionValue :type Boolean) (ElapsedSeconds :type "Float (double-precision)") (TriggeredSeconds :type "Float (double-precision)") (InputAction :type "InputAction Object Reference" :default "/Game/BP/Inputs/InputActions/IA_ToogleInventory.IA_ToogleInventory"))
  ;[0.04167 0.04167 0.04167] ToogleInventory
  (:`Triggered`
    (`/Game/BP/HUDs/BaseHUD.ke_ToogleInventory` (`self.HUDRef`) true)))

(event `EnhancedInput|/Game/BP/Inputs/InputActions/IA_Run`
  (params (ActionValue :type Boolean) (ElapsedSeconds :type "Float (double-precision)") (TriggeredSeconds :type "Float (double-precision)") (InputAction :type "InputAction Object Reference" :default "/Game/BP/Inputs/InputActions/IA_Run.IA_Run"))
  (bind _playerstats (`self.PlayerStats`))
  (bind _playerstats_2 (`self.PlayerStats`))
  ;[0.04167 0.04167 0.04167] Run
  (:`Triggered`
    (if (`/Game/BP/Components/PlayerStats.HasEnoughStamina?` _playerstats)
      (`self.UpdateSpeedOnServer` (`self.OwnerRef`) (`self.RunSpeed`))
      (if (> (`KismetMathLibrary.VSizeXY` (`self.GetVelocity` (`self.OwnerRef`))) 10.0)
        (`/Game/BP/Components/PlayerStats.ToogleRun` _playerstats_2 true 0.1)
        (else
          (`/Game/BP/Components/PlayerStats.ToogleRun` _playerstats_2 false 0.0)))
      (else
        (`self.UpdateSpeedOnServer` (`self.OwnerRef`) (`self.WalkSpeed`) :!label _label_2))))
  (:`Canceled`
    (`/Game/BP/Components/PlayerStats.ToogleRun` _playerstats false 0.0 :!label _label_3)
    (goto _label_2))
  (:`Completed`
    (goto _label_3)))

(event `UpdateSpeedOnServer`
  (params (Target :type "Character Object Reference") (`Max Walk Speed` :type "Float (single-precision)"))
  ;[0.04167 0.04167 0.04167] Run
  (`self.UpdateSpeedMulticast` Target `Max Walk Speed`))

(event `UpdateSpeedMulticast`
  (params (Target :type "Character Object Reference") (`Max Walk Speed` :type "Float (single-precision)"))
  ;[0.04167 0.04167 0.04167] Run
  (set `CharacterMovementComponent.MaxWalkSpeed` `Max Walk Speed` (`Character.CharacterMovement` Target)))

(event `self.ReceiveBeginPlay`
  (bind _returnvalue (subsystem `EnhancedInputLocalPlayerSubsystem`))
  ;[0.04167 0.04167 0.04167] Setup Reference and start mapping input
  (`/Engine/EditorBlueprintResources/StandardMacros.IsValid` _returnvalue
    (:`Is Valid`
      (`EnhancedInputSubsystemInterface.AddMappingContext` _returnvalue "/Game/BP/Inputs/MappingContexts/IMC_Player.IMC_Player" 0 (struct))
      (bind _asbp_player (cast `/Game/BP/Character/PlayerCharacter/BP_Player` (`self.K2_GetPawn`)))
      (set `self.OwnerRef` _asbp_player)
      (bind _asbase_hud (cast `/Game/BP/HUDs/BaseHUD` (`self.GetHUD`)))
      (set `self.HUDRef` _asbase_hud))))

(fn `AimTraceFromPlayer`
  (params (TraceLength :type "Float (single-precision)" :default 400.0) (Radius :type "Float (single-precision)" :default 6.0) (DrawDebugType :type "EDrawDebugTrace Enum" :default "None") (DrawTime :type "Float (single-precision)" :default 0.01))
  (returns (ReturnValue :type Boolean) (OutHit :type "HitResult Structure"))
  (bind _returnvalue (`GameplayStatics.GetPlayerCameraManager` 0))
  (bind _returnvalue_2 (`PlayerCameraManager.GetCameraLocation` _returnvalue))
  (bind (_outhit _returnvalue_3) (`KismetSystemLibrary.SphereTraceSingle` :`Start` _returnvalue_2 :`End` (+ _returnvalue_2 (* (`self.GetActorForwardVector` _returnvalue) TraceLength)) :`Radius` Radius :`TraceChannel` "TraceTypeQuery1" :`DrawDebugType` DrawDebugType :`DrawTime` DrawTime))
  (return _returnvalue_3 _outhit))

(fn `UserConstructionScript`)