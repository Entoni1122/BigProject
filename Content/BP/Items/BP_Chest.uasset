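; BP_Chest is an interactable chest item that holds randomly generated loot.
; On BeginPlay it picks a random item count and fills its Items array with random rows from DT_RandomChest, with repeats possible.
; A TableId select feeds the row-name lookup, though both options point to the same table.
; Interacting through I_Interact passes Items to the HUD main widget's ToggleChest and returns false.
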(event `self.ReceiveBeginPlay`
  (bind _output_get (set `self.RandomAmountItem` (`KismetMathLibrary.RandomIntegerInRange` 2 5)))
  (bind _outrownames (`DataTableFunctionLibrary.GetDataTableRowNames` (select `int` (`self.TableId`) :`0` "/Game/BP/Datatables/DT_RandomChest.DT_RandomChest" :`1` "/Game/BP/Datatables/DT_RandomChest.DT_RandomChest" :!type "DataTable Object Reference")))
  (for _ (range _output_get)
    (bind _returnvalue (`|GetDataTableRow` "/Game/BP/Datatables/DT_RandomChest.DT_RandomChest" (`KismetArrayLibrary.Array_Random` _outrownames))
      (:`then`
        (`KismetArrayLibrary.Array_Add` (`self.Items`) _returnvalue)))))

(fn `I_Interact`
  (returns (`Item?` :type Boolean))
  (`/Game/BP/Widgets/WDB_HUD.ToggleChest` (`/Game/BP/HUDs/BaseHUD.MainWidgetRef` (`/Game/BP/Functions/CustomLibrary.GetHUD`)) (`self.Items`))
  (return false))

(fn `UserConstructionScript`)