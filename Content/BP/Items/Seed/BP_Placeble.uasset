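; BP_Placeble is a placeable item Actor that swaps its mesh material while its collision check component overlaps another actor.
; BeginPlay turns off physics, then overlap begin applies M_PlaceItem and any overlap end restores Chest1, without counting overlaps.
; It implements I_Interact with a stub that only returns true.
; Debug prints show overlapping actor names and, every tick, the current material.
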(event `self.ReceiveBeginPlay`
  (`PrimitiveComponent.SetSimulatePhysics` (`self.StaticMeshComponent`) false))

(event `self.CheckForCollision.OnComponentBeginOverlap`
  (params (OverlappedComponent :type "PrimitiveComponent Object Reference") (OtherActor :type "Actor Object Reference") (OtherComp :type "PrimitiveComponent Object Reference") (OtherBodyIndex :type Integer) (bFromSweep :type Boolean) (SweepResult :type "HitResult Structure (by ref)"))
  (`KismetSystemLibrary.PrintString` (`KismetSystemLibrary.GetDisplayName` OtherActor))
  (`PrimitiveComponent.SetMaterial` (`self.StaticMeshComponent`) 0 "/Game/Materials/M_PlaceItem.M_PlaceItem"))

(event `self.CheckForCollision.OnComponentEndOverlap`
  (params (OverlappedComponent :type "PrimitiveComponent Object Reference") (OtherActor :type "Actor Object Reference") (OtherComp :type "PrimitiveComponent Object Reference") (OtherBodyIndex :type Integer))
  (`KismetSystemLibrary.PrintString` (`KismetSystemLibrary.GetDisplayName` OtherActor))
  (`PrimitiveComponent.SetMaterial` (`self.StaticMeshComponent`) 0 "/Game/BP/Items/Chest/chest1.chest1"))

(event `self.ReceiveTick`
  (params (DeltaSeconds :type "Float (single-precision)"))
  (`KismetSystemLibrary.PrintString` (`KismetSystemLibrary.GetDisplayName` (`PrimitiveComponent.GetMaterial` (`self.StaticMeshComponent`) 0)) true true (struct :`G` 0.66 :`B` 1.0 :`A` 1.0) 2.0 "1212"))

(fn `I_Interact`
  (returns (`Item?` :type Boolean))
  (return true))

(fn `UserConstructionScript`
  (`parent.UserConstructionScript`))